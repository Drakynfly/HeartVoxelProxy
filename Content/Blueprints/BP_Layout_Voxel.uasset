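; BP_Layout_Voxel is a Heart graph layout helper that automatically arranges nodes into layered trees.
; It resolves the given nodes, filters out annotations, and sorts the rest into trees along output connections, allowing duplicates.
; Each tree becomes layers stepped toward negative X, with nodes stacked along Y and each tree offset by a fixed spacing.
; Positions are written through the graph interface, and a debug message prints on completion.
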(fn `Layout_BP`
  (params (Interface :type "HeartGraphInterface Interface (by ref)") (Nodes :type "Array of HeartNodeGuid Structure (by ref)"))
  (returns (ReturnValue :type Boolean))
  (bind _returnvalue (`HeartNodeSortingLibrary.ResolveNodes` (`HeartGraphInterface.GetHeartGraph` Interface) Nodes))
  (bind _returnvalue_2 (`HeartNodeSortingLibrary.FilterNodesByClass_Exclusive` _returnvalue (`|MakeSet` "/Script/Heart.HeartGraphNodeAnnotation" :!type "HeartGraphNode Class Reference")))
  (bind _trees (`HeartNodeSortingLibrary.SortLooseNodesIntoTrees` _returnvalue_2 (make `NodeLooseToTreeArgs` true "Output")))
  (for (_array_element _array_index) _trees
    (bind _layers (`HeartNodeSortingLibrary.ConvertNodeTreeToLayers` _array_element))
    (for (_array_element_2 _array_index_2) _layers
      (bind _result (`BlueprintSetLibrary.Set_ToArray` (`.Nodes` (break `HeartNodeLayer` _array_element_2))))
      (for (_array_element_3 _array_index_3) _result
        (`HeartGraphInterface.SetNodeLocation` (`local.Interface`) _array_element_3 (`KismetMathLibrary.MakeVector2D` (* _array_index_2 (`self.LayerSpacing`) -1.0) (+ (* _array_index_3 (`self.NodeSpacing`)) (* _array_index (`self.TreeSpacing`)))) false))))
  (`KismetSystemLibrary.PrintString` self "LayoutHelper End")
  (return true))